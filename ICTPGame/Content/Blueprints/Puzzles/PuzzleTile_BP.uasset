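; PuzzleTile_BP is a puzzle floor tile that can damage players and reveal itself as harmful.
; On switch activation it shows the ParentDummy hierarchy only if ShowColour and DoesDamage are both set.
; HitBox overlap by a registered robot player's pawn calls the game mode's TryDamage and reveals ParentDummy on damaging tiles; ending overlap hides it.
; ParentDummy starts hidden; an older dynamic-material colour approach remains disconnected.
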(event `OnSwitchActivation`
  ;[1 1 1] Show Colour
  (if (`self.showColour`)
    (if (`self.doesDamage`)
      (`SceneComponent.SetVisibility` (`self.ParentDummy`) true true)
      (else
        (`SceneComponent.SetVisibility` (`self.ParentDummy`) false true)))
    (else
      (`SceneComponent.SetVisibility` (`self.ParentDummy`) false true))))

(event `self.HitBox.OnComponentBeginOverlap`
  (params (OtherActor :type "Actor Object Reference") (OtherComp :type "PrimitiveComponent Object Reference") (OtherBodyIndex :type Integer) (bFromSweep :type Boolean) (SweepResult :type "HitResult Structure (by ref)"))
  ;[1 1 1] Damage Player
  (bind _asictpgame_game_mode (cast `ICTPGameGameMode` (`GameplayStatics.GetGameMode`)))
  (bind _aspawn (cast `Pawn` OtherActor))
  (bind _asrobot_player_controller (cast `RobotPlayerController` (`self.GetController` _aspawn)))
  (if (`KismetArrayLibrary.Array_Contains` (`ICTPGameGameMode.Players` _asictpgame_game_mode) _asrobot_player_controller)
    (if (`self.doesDamage`)
      (`ICTPGameGameMode.TryDamage` _asictpgame_game_mode self OtherActor 15.0 null)
      (`SceneComponent.SetVisibility` (`self.ParentDummy`) true true)
      (else
        (`SceneComponent.SetVisibility` (`self.ParentDummy`) false true)))))

(event `self.HitBox.OnComponentEndOverlap`
  (params (OtherActor :type "Actor Object Reference") (OtherComp :type "PrimitiveComponent Object Reference") (OtherBodyIndex :type Integer))
  ;[1 1 1] Return Colour to Blue
  (`SceneComponent.SetVisibility` (`self.ParentDummy`) false true))

(fn `UserConstructionScript`
  (`SceneComponent.SetVisibility` (`self.ParentDummy`) false true))