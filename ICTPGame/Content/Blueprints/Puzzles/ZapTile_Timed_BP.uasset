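; Timed electric floor tile hazard that cycles between idle, flashing warning and zapping states while DoesDamage is set.
; After a startup Delay, Tick accumulates wait time, then flickers ParentDummy's visibility and switches ZapOn for OnTime, using Delay nodes and start/loop sounds.
; HitBox begin-overlap during a zap sends damage for registered robot players through the game mode's TryDamage.
; OnSwitchActivation syncs tile visibility to DoesDamage.
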(event `OnSwitchActivation`
  ;[1 1 1] Show Colour
  (if (`self.doesDamage`)
    (`SceneComponent.SetVisibility` (`self.ParentDummy`) true true)
    (else
      (`SceneComponent.SetVisibility` (`self.ParentDummy`) false true))))

(event `self.ReceiveBeginPlay`
  (`KismetSystemLibrary.Delay` (`self.Delay`))
  (set `self.Go` true))

(event `self.ReceiveTick`
  (params (DeltaSeconds :type "Float (single-precision)"))
  (bind _ambientstartsound (`self.AmbientStartSound`))
  (bind _ambientloopsound (`self.AmbientLoopSound`))
  ;[1 1 1] Start Flashing
  (if (and (`self.doesDamage`) (`self.Go`))
    (if (`self.ZapOn`)
      ;[1 1 1] Set Visibility for Damage Period
      (`SceneComponent.SetVisibility` (`self.ParentDummy`) true true)
      (`KismetSystemLibrary.Delay` (`self.OnTime`))
      (set `self.CurrentTime` 0.0)
      (set `self.ZapOn` false)
      (`SceneComponent.SetVisibility` (`self.ParentDummy`) false true)
      (`/Engine/EditorBlueprintResources/StandardMacros.IsValid` _ambientloopsound
        (:`Is Valid`
          (`AudioComponent.FadeOut` _ambientloopsound 0.5 0.0)
          (set `self.AmbientLoopSound` null)))
      (else
        (bind _output_get (set `self.CurrentTime` (+ DeltaSeconds (`self.CurrentTime`))))
        (if (> _output_get (`self.WaitInterval`))
          (if (not (`KismetSystemLibrary.IsValid` (`self.AmbientStartSound`)))
            (bind _returnvalue (`GameplayStatics.SpawnSoundAttached` "/Game/Audio/Sounds/Environment/Tiles/Electric_Plate_Start_2.Electric_Plate_Start_2" (`self.DefaultSceneRoot`)))
            (set `self.AmbientStartSound` _returnvalue))
          (`KismetSystemLibrary.Delay` 0.1)
          (`self.Flash`)
          (if (> (`self.CurrentTime`) (+ (`self.WaitInterval`) (`self.FlashTime`)))
            (set `self.ZapOn` true)
            (`/Engine/EditorBlueprintResources/StandardMacros.IsValid` _ambientstartsound
              (:`Is Valid`
                (`AudioComponent.FadeOut` _ambientstartsound 0.5 0.0))
              (:`Is Not Valid`
                (set `self.AmbientStartSound` _ambientstartsound)
                (bind _returnvalue_2 (`GameplayStatics.SpawnSoundAttached` "/Game/Audio/Sounds/Environment/Tiles/Electric_Plate_Loop_2.Electric_Plate_Loop_2" (`self.DefaultSceneRoot`)))
                (set `self.AmbientLoopSound` _returnvalue_2)))))))))

(event `self.HitBox.OnComponentBeginOverlap`
  (params (OtherActor :type "Actor Object Reference") (OtherComp :type "PrimitiveComponent Object Reference") (OtherBodyIndex :type Integer) (bFromSweep :type Boolean) (SweepResult :type "HitResult Structure (by ref)"))
  ;[1 1 1] Damage Player
  (if (`self.ZapOn`)
    (bind _asictpgame_game_mode (cast `ICTPGameGameMode` (`GameplayStatics.GetGameMode`)))
    (bind _aspawn (cast `Pawn` OtherActor))
    (bind _asrobot_player_controller (cast `RobotPlayerController` (`self.GetController` _aspawn)))
    (if (`KismetArrayLibrary.Array_Contains` (`ICTPGameGameMode.Players` _asictpgame_game_mode) _asrobot_player_controller)
      (if (`self.doesDamage`)
        (`ICTPGameGameMode.TryDamage` _asictpgame_game_mode self OtherActor 15.0 null)))))

(fn `Flash`
  (bind _output_get (set `self.Visibility` (not (`self.Visibility`))))
  (`SceneComponent.SetVisibility` (`self.ParentDummy`) _output_get true))

(fn `UserConstructionScript`
  (`SceneComponent.SetVisibility` (`self.ParentDummy`) false true))