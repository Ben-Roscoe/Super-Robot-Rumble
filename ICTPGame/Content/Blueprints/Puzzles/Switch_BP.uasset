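; Switch_BP is a puzzle switch that is active while a player robot stands in its collision box.
; Begin overlap sets IsActive only for a pawn whose RobotPlayerController_BP is in the ICTPGameGameMode Players list.
; End overlap clears IsActive unconditionally, without checking which actor left or whether others remain inside.
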(event `self.ReceiveBeginPlay`)

(event `self.ReceiveActorBeginOverlap`
  (params (OtherActor :type "Actor Object Reference")))

(event `self.ReceiveTick`
  (params (DeltaSeconds :type "Float (single-precision)")))

(event `self.collisionBox.OnComponentBeginOverlap`
  (params (OtherActor :type "Actor Object Reference") (OtherComp :type "PrimitiveComponent Object Reference") (OtherBodyIndex :type Integer) (bFromSweep :type Boolean) (SweepResult :type "HitResult Structure (by ref)"))
  (bind _asictpgame_game_mode (cast `ICTPGameGameMode` (`GameplayStatics.GetGameMode`)))
  (bind _aspawn (cast `Pawn` OtherActor))
  (bind _asrobot_player_controller_bp (cast `/Game/Blueprints/RobotPlayerController_BP` (`self.GetController` _aspawn)))
  (if (`KismetArrayLibrary.Array_Contains` (`ICTPGameGameMode.Players` _asictpgame_game_mode) _asrobot_player_controller_bp)
    (set `self.isActive` true)))

(event `self.collisionBox.OnComponentEndOverlap`
  (params (OtherActor :type "Actor Object Reference") (OtherComp :type "PrimitiveComponent Object Reference") (OtherBodyIndex :type Integer))
  (set `self.isActive` false))

(fn `UserConstructionScript`)