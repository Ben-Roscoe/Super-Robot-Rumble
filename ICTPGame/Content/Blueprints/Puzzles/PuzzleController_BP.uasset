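; PuzzleController_BP is a puzzle controller that reveals tile colours while any switch is active.
; Its construction script gathers every PuzzleTile_BP and Switch_BP actor through GetAllActorsOfClass.
; Each Tick it scans the switches, sets ShowColour on all tiles and calls their OnSwitchActivation.
; That call repeats every frame while a switch is active, whereas a TilesAreActive flag limits switching off to one pass.
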(event `self.ReceiveTick`
  (params (DeltaSeconds :type "Float (single-precision)"))
  (bind _switches (`self.switches`))
  (bind _tilearray (`self.tileArray`))
  (if (> (`KismetArrayLibrary.Array_Length` _switches) 0)
    (for _array_element _switches
      (if (`/Game/Blueprints/Puzzles/Switch_BP.isActive` _array_element)
        (set `self.SwitchIsActive` true)
        (break)
        (else
          (set `self.SwitchIsActive` false))))
    (if (`self.SwitchIsActive`)
      (for _array_element_2 _tilearray
        (set `/Game/Blueprints/Puzzles/PuzzleTile_BP.showColour` true _array_element_2)
        (set `self.TilesAreActive` true)
        (`/Game/Blueprints/Puzzles/PuzzleTile_BP.OnSwitchActivation` _array_element_2))
      (elif (`self.TilesAreActive`)
        (for _array_element_3 _tilearray
          (set `/Game/Blueprints/Puzzles/PuzzleTile_BP.showColour` false _array_element_3)
          (set `self.TilesAreActive` false)
          (`/Game/Blueprints/Puzzles/PuzzleTile_BP.OnSwitchActivation` _array_element_3))))))

(fn `UserConstructionScript`
  (bind _outactors (`GameplayStatics.GetAllActorsOfClass` "/Game/Blueprints/Puzzles/PuzzleTile_BP.PuzzleTile_BP_C"))
  (set `self.tileArray` _outactors)
  (bind _outactors_2 (`GameplayStatics.GetAllActorsOfClass` "/Game/Blueprints/Puzzles/Switch_BP.Switch_BP_C"))
  (set `self.switches` _outactors_2))