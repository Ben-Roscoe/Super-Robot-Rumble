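; Pistol bullet projectile actor tinted with the colour of the RobotPlayerController that fired it.
; A dynamic material instance created at construction receives that colour on BeginPlay via the instigator controller.
; When its Box hits something, it passes damage through ICTPGameGameMode's TryDamage, spawns a reverse-yawed laser damage emitter in the same colour, and destroys itself.
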(event `self.ReceiveBeginPlay`
  (bind _asrobot_player_controller (cast `RobotPlayerController` (`self.GetInstigatorController`)))
  (`MaterialInstanceDynamic.SetVectorParameterValue` (`self.Material Instance`) "BulletColour" (`KismetMathLibrary.Conv_ColorToLinearColor` (`RobotPlayerController.GetColour` _asrobot_player_controller))))

(event `self.ReceiveActorBeginOverlap`
  (params (OtherActor :type "Actor Object Reference")))

(event `self.ReceiveTick`
  (params (DeltaSeconds :type "Float (single-precision)")))

(event `self.Box.OnComponentHit`
  (params (OtherActor :type "Actor Object Reference") (OtherComp :type "PrimitiveComponent Object Reference") (NormalImpulse :type "Vector Structure") (Hit :type "HitResult Structure (by ref)"))
  (bind (_returnvalue_roll _returnvalue_pitch _returnvalue_yaw) (`KismetMathLibrary.BreakRotator` (`self.K2_GetActorRotation` self)))
  (bind _asictpgame_game_mode (cast `ICTPGameGameMode` (`GameplayStatics.GetGameMode`)))
  (`ICTPGameGameMode.TryDamage` _asictpgame_game_mode self OtherActor 10.0 null)
  (bind _returnvalue (`GameplayStatics.SpawnEmitterAtLocation` "/Game/Particles/P_LaserDamage.P_LaserDamage" (`SceneComponent.K2_GetComponentLocation` (`self.StaticMesh`)) (`KismetMathLibrary.MakeRotator` _returnvalue_roll _returnvalue_pitch (+ _returnvalue_yaw 180.0)) false))
  (`ParticleSystemComponent.SetColorParameter` _returnvalue "ParticleBlocksColour" (`KismetMathLibrary.Conv_ColorToLinearColor` (`RobotPlayerController.GetColour` (stale `self.ReceiveBeginPlay` _asrobot_player_controller))))
  (`self.K2_DestroyActor`))

(fn `UserConstructionScript`
  (bind _returnvalue (`PrimitiveComponent.CreateDynamicMaterialInstance` (`self.StaticMesh`) 0 null))
  (set `self.Material Instance` _returnvalue))