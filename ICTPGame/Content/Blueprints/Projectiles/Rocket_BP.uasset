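; Bouncing rocket projectile that explodes on hitting an actor with a HealthComponent, or on any other hit once it reaches its bounce limit.
; The box collider ignores the instigator when moving, and the projectile movement component's bounce event counts bounces.
; Exploding requests radial damage through the ICTPGameGameMode, spawns an effect scaled to the ExplosionRadius sphere, plays a sound and destroys the rocket.
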(event `self.ReceiveBeginPlay`
  (`PrimitiveComponent.IgnoreActorWhenMoving` (`self.Box`) (`self.Instigator`) true))

(event `self.Box.OnComponentHit`
  (params (OtherActor :type "Actor Object Reference") (OtherComp :type "PrimitiveComponent Object Reference") (NormalImpulse :type "Vector Structure") (Hit :type "HitResult Structure (by ref)"))
  (`/Engine/EditorBlueprintResources/StandardMacros.IsValid` OtherActor
    (:`Is Valid`
      (bind _outcomponent (`/Game/Blueprints/Libraries/Utilities.GetComponentByClass` "/Script/ICTPGame.HealthComponent" OtherActor))
      (`/Engine/EditorBlueprintResources/StandardMacros.IsValid` _outcomponent
        (:`Is Valid`
          (`self.Explode` :!label _label))
        (:`Is Not Valid`
          (if (>= (`self.Bounces`) (`self.MaxBounces`)) :!label _label_2
            (goto _label)))))
    (:`Is Not Valid`
      (goto _label_2))))

(event `self.ProjectileMovement.OnProjectileBounce`
  (params (ImpactResult :type "HitResult Structure (by ref)") (ImpactVelocity :type "Vector Structure (by ref)"))
  (`/Engine/EditorBlueprintResources/StandardMacros.IncrementInt` (`self.Bounces`)))

(fn `Explode`
  (bind _returnvalue (`SceneComponent.K2_GetComponentLocation` (`self.ExplosionRadius`)))
  (bind _asictpgame_game_mode (cast `ICTPGameGameMode` (`GameplayStatics.GetGameMode`)))
  (`ICTPGameGameMode.TryRadialDamage` _asictpgame_game_mode self (`self.Damage`) (`SphereComponent.SphereRadius` (`self.ExplosionRadius`)) _returnvalue "/Script/Engine.DamageType")
  (bind _returnvalue_2 (`GameplayStatics.SpawnEmitterAtLocation` "/Game/Particles/P_Explosion_Yellow.P_Explosion_Yellow" _returnvalue (struct) false))
  (`SceneComponent.SetRelativeScale3D` _returnvalue_2 (`KismetMathLibrary.Conv_DoubleToVector` (/ (`SphereComponent.SphereRadius` (`self.ExplosionRadius`)) (`self.DefaultExplosionSize`))))
  (`GameplayStatics.PlaySoundAtLocation` "/Game/Audio/Sounds/Weapons/RocketLauncher/Rocket_Explosion.Rocket_Explosion" (`self.K2_GetActorLocation`))
  (`self.K2_DestroyActor`))

(fn `UserConstructionScript`)