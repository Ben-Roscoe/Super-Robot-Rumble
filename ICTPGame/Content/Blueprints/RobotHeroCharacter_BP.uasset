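; Player robot hero character Blueprint that takes its colour from the controller, mounts weapons and explodes on death.
; The construction script creates dynamic materials for the mesh and lower body, shared with the flash-on-damage component and tinted on possession.
; Created weapons attach to the mesh's weapon socket, and damage plays an attached sound.
; On death it spawns an explosion effect and asks the game mode to apply radial damage.
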(event `self.ReceivePossessed`
  (params (NewController :type "Controller Object Reference"))
  (for _array_element (`self.MaterialInstanceArray`)
    (bind _asmaterial_instance_dynamic (cast `MaterialInstanceDynamic` _array_element))
    (bind _asrobot_player_controller (cast `RobotPlayerController` (`self.GetController`)))
    (`MaterialInstanceDynamic.SetVectorParameterValue` _asmaterial_instance_dynamic "PlayerColour" (`KismetMathLibrary.Conv_ColorToLinearColor` (`RobotPlayerController.GetColour` _asrobot_player_controller)))))

(event `self.MultipleWeaponUserComponent.OnWeaponCreated`
  (params (Weapon :type "WeaponActor Object Reference"))
  (`self.K2_AttachRootComponentTo` Weapon (`self.Mesh`) "WeaponSocket" "SnapToTargetIncludingScale" true))

(event `self.HealthComponent.OnDeath`
  (params (DamageAmount :type "Float (single-precision)") (Instigator :type "Controller Object Reference") (DamageCauser :type "Actor Object Reference"))
  (bind _explosionradius (`self.ExplosionRadius`))
  (`GameplayStatics.SpawnEmitterAtLocation` "/Game/Particles/P_Explosion_Yellow.P_Explosion_Yellow" (`SceneComponent.K2_GetComponentLocation` (`self.CapsuleComponent`)))
  (bind _asictpgame_game_mode (cast `ICTPGameGameMode` (`GameplayStatics.GetGameMode`)))
  (`ICTPGameGameMode.TryRadialDamage` _asictpgame_game_mode self (`self.ExplosionDamage`) (`SphereComponent.SphereRadius` _explosionradius) (`SceneComponent.K2_GetComponentLocation` _explosionradius) "/Script/Engine.DamageType"))

(event `self.ReceiveBeginPlay`
  (add `self.OnTakeAnyDamage` (delegate `TakeDamage`)))

(event `TakeDamage` :!signature `self.OnTakeAnyDamage`
  (params (Damage :type "Float (double-precision)") (DamageType :type "DamageType Object Reference") (InstigatedBy :type "Controller Object Reference") (DamageCauser :type "Actor Object Reference"))
  (`GameplayStatics.SpawnSoundAttached` "/Game/Audio/Sounds/Player/Player_Take_Damage_2.Player_Take_Damage_2" (`self.CapsuleComponent`)))

(fn `UserConstructionScript`
  (bind _materialinstancearray (`self.MaterialInstanceArray`))
  (bind _returnvalue (`PrimitiveComponent.CreateDynamicMaterialInstance` (`self.Mesh`) 0 null))
  (`KismetArrayLibrary.Array_Add` _materialinstancearray _returnvalue)
  (bind _returnvalue_2 (`PrimitiveComponent.CreateDynamicMaterialInstance` (`self.Mesh`) 1 null))
  (`KismetArrayLibrary.Array_Add` _materialinstancearray _returnvalue_2)
  (bind _returnvalue_3 (`PrimitiveComponent.CreateDynamicMaterialInstance` (`self.LowerBody`) 0 null))
  (`KismetArrayLibrary.Array_Add` _materialinstancearray _returnvalue_3)
  (for _array_element (`self.MaterialInstanceArray`)
    (`KismetArrayLibrary.Array_Add` (`/Game/Blueprints/Components/FlashOnDamageComponent_BP.FlashMaterials` (`self.FlashOnDamageComponent_BP`)) _array_element)))