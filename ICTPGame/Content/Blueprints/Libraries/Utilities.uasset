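; Utilities is a function library with two general helpers for actor queries.
; GetClosestActor loops over an actor array, tracking the one whose location has the smallest distance to a given origin below the running ClosestDistance.
; GetComponentByClass returns the first component of a given class on an actor, or nothing when the actor has none.
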(fn GetClosestActor
  (params (Actors :type Array%20of%20Actor%20Object%20References) (Origin :type Vector))
  (for _array_element Actors
    (if (< (Math|Vector|VectorLength (- (Transformation|GetActorLocation _array_element) Origin)) (LocalVariables|GetClosestDistance))
      (LocalVariables|SetClosestDistance (Math|Vector|VectorLength (- (Transformation|GetActorLocation _array_element) Origin)))
      (LocalVariables|SetCurrentClosestActor _array_element)))
  (return (LocalVariables|GetCurrentClosestActor)))

(fn GetComponentbyClass
  (params (Class :type Actor%20Component%20Class%20Reference) (Actor :type Actor%20Object%20Reference))
  (bind _returnvalue (Actor|GetComponentsByClass Actor Class))
  (if (> (Utilities|Array|Length _returnvalue) 0)
    (return (Utilities|Array|Get(acopy) _returnvalue))
    (else
      (return 0))))