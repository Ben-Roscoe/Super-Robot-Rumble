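; Rocket launcher weapon that launches a Rocket_BP projectile when its FireWeapon event runs.
; It spawns the rocket at a fire-origin transform derived from the Arrow component, passes on its Instigator and plays the firing sound at the actor's location.
; A timeline then drives a rotator lerp that turns the Grenades component through a relative rotation toward 120 degrees on each shot.
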(event `self.ReceiveBeginPlay`)

(event `self.ReceiveActorBeginOverlap`
  (params (OtherActor :type "Actor Object Reference")))

(event `self.ReceiveTick`
  (params (DeltaSeconds :type "Float (single-precision)")))

(event `self.FireWeapon`
  (`|SpawnActorFromClass` "/Game/Blueprints/Projectiles/Rocket_BP.Rocket_BP_C" (`KismetMathLibrary.MakeTransform` (`self.WorldLocationToFireOriginLocation` (`SceneComponent.RelativeLocation` (`self.Arrow`))) (`self.WorldRotationToFireOriginRotation` (`SceneComponent.RelativeRotation` (`self.Arrow`)))) "Undefined" "OverrideRootScale" null (`self.GetInstigator`))
  (`GameplayStatics.PlaySoundAtLocation` "/Game/Audio/Sounds/Weapons/RocketLauncher/Rocket_Fire.Rocket_Fire" (`self.K2_GetActorLocation`))
  (bind (_direction _lerptime) (`Timeline|Timeline_0`)
    (:`Update`
      (`SceneComponent.K2_SetRelativeRotation` (`self.Grenades`) (`KismetMathLibrary.RLerp` (struct) (struct :`Roll` 120.0) _lerptime) false false))))

(fn `UserConstructionScript`)