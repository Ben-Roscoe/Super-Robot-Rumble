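; Shotgun weapon Blueprint that fires a three-projectile spread with a firing sound.
; FireWeapon calls SpawnProjectile for the Left, Middle and Right arrow components, then plays the Shotgun sound at the actor's location.
; SpawnProjectile spawns a PistolBullet_BP, passing the arrow's relative location and rotation through fire-origin conversion functions and forwarding the weapon's Instigator.
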(event `self.ReceiveBeginPlay`)

(event `self.ReceiveActorBeginOverlap`
  (params (OtherActor :type "Actor Object Reference")))

(event `self.ReceiveTick`
  (params (DeltaSeconds :type "Float (single-precision)")))

(event `self.FireWeapon`
  (`self.SpawnProjectile` (`self.Left`))
  (`self.SpawnProjectile` (`self.Middle`))
  (`self.SpawnProjectile` (`self.Right`))
  (`GameplayStatics.PlaySoundAtLocation` "/Game/Audio/Sounds/Weapons/Shotgun/Shotgun.Shotgun" (`self.K2_GetActorLocation`)))

(fn `SpawnProjectile`
  (params (ArrowComponent :type "ArrowComponent Object Reference"))
  (`|SpawnActorFromClass` "/Game/Blueprints/Projectiles/PistolBullet_Bp.PistolBullet_BP_C" (`KismetMathLibrary.MakeTransform` (`self.WorldLocationToFireOriginLocation` (`SceneComponent.RelativeLocation` ArrowComponent)) (`self.WorldRotationToFireOriginRotation` (`SceneComponent.RelativeRotation` ArrowComponent)) (`SceneComponent.K2_GetComponentScale` ArrowComponent)) "Undefined" "OverrideRootScale" null (`self.GetInstigator`)))

(fn `UserConstructionScript`)