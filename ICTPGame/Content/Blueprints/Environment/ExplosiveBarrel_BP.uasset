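; Explosive barrel actor that blows up and deals radial damage when its Health component fires OnDeath.
; It asks ICTPGameGameMode to apply the damage at the barrel's location, using the ExplosionRadius sphere as the blast range.
; It then spawns an explosion particle scaled by that radius relative to DefaultExplosionRadius, plays a sound and destroys itself.
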(event `self.ReceiveBeginPlay`)

(event `self.ReceiveActorBeginOverlap`
  (params (OtherActor :type "Actor Object Reference")))

(event `self.ReceiveTick`
  (params (DeltaSeconds :type "Float (single-precision)")))

(event `self.Health.OnDeath`
  (params (DamageAmount :type "Float (single-precision)") (Instigator :type "Controller Object Reference") (DamageCauser :type "Actor Object Reference"))
  (bind _returnvalue (`self.K2_GetActorLocation`))
  (bind _asictpgame_game_mode (cast `ICTPGameGameMode` (`GameplayStatics.GetGameMode`)))
  (`ICTPGameGameMode.TryRadialDamage` _asictpgame_game_mode self (`self.Damage`) (`SphereComponent.SphereRadius` (`self.ExplosionRadius`)) _returnvalue "/Script/Engine.DamageType")
  (bind _returnvalue_2 (`GameplayStatics.SpawnEmitterAtLocation` "/Game/Particles/P_Explosion_Yellow.P_Explosion_Yellow" _returnvalue))
  (`SceneComponent.SetRelativeScale3D` _returnvalue_2 (`KismetMathLibrary.Conv_DoubleToVector` (/ (`SphereComponent.SphereRadius` (`self.ExplosionRadius`)) (`self.DefaultExplosionRadius`))))
  (`GameplayStatics.PlaySoundAtLocation` "/Game/Audio/Sounds/Weapons/RocketLauncher/Rocket_Explosion.Rocket_Explosion" (`self.K2_GetActorLocation`))
  (`self.K2_DestroyActor`))

(fn `UserConstructionScript`)