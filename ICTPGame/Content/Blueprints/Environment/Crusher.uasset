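; Environmental crusher hazard that slides its plate along local X and damages actors caught in its damage area.
; After a start delay, Tick plays the Crush timeline while CanCrush is set, lerping the plate's relative location.
; Damage is enabled only while the plate trigger overlaps a Crusher's plate trigger, such as an opposing plate.
; Each enabled tick sends overlapping actors to the game mode's TryDamage.
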(event `self.ReceiveBeginPlay`
  ;[1 1 1] StartDelay
  (`KismetSystemLibrary.Delay` (`self.StartDelay`))
  (set `self.CanStart` true))

(event `self.ReceiveTick`
  (params (DeltaSeconds :type "Float (single-precision)"))
  (if (`self.CanStart`)
    (`|ExecutionSequence`
      (:`then_0`
        (if (`self.CanCrush`)
          (bind (_direction _newtrack_0) (`Timeline|Crush`)
            (:`Update`
              (`SceneComponent.K2_SetRelativeLocation` (`self.CrusherPlate`) (`KismetMathLibrary.VLerp` (0.0 0.0 0.0) (140.0 0.0 0.0) _newtrack_0) false false)))))
      (:`then_1`
        (if (`self.IsDamageEnabled`)
          (for _array_element (`PrimitiveComponent.GetOverlappingActors` (`self.CrushPlateDamageArea`) "/Script/Engine.Actor")
            (bind _asictpgame_game_mode (cast `ICTPGameGameMode` (`GameplayStatics.GetGameMode`)))
            (`ICTPGameGameMode.TryDamage` _asictpgame_game_mode self _array_element (`self.CrushingDamage`) "/Script/Engine.DamageType")))))))

(event `self.CrusherPlateTrigger.OnComponentBeginOverlap`
  (params (OtherActor :type "Actor Object Reference") (OtherComp :type "PrimitiveComponent Object Reference") (OtherBodyIndex :type Integer) (bFromSweep :type Boolean) (SweepResult :type "HitResult Structure (by ref)"))
  (bind _ascrusher (cast `/Game/Blueprints/Environment/Crusher` OtherActor))
  (if (== (`/Game/Blueprints/Environment/Crusher.CrusherPlateTrigger` _ascrusher) OtherComp)
    (set `self.IsDamageEnabled` true)))

(event `self.CrusherPlateTrigger.OnComponentEndOverlap`
  (params (OtherActor :type "Actor Object Reference") (OtherComp :type "PrimitiveComponent Object Reference") (OtherBodyIndex :type Integer))
  (bind _ascrusher (cast `/Game/Blueprints/Environment/Crusher` OtherActor))
  (if (== (`/Game/Blueprints/Environment/Crusher.CrusherPlateTrigger` _ascrusher) OtherComp)
    (set `self.IsDamageEnabled` false)))

(fn `UserConstructionScript`)