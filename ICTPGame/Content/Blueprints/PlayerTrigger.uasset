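; One-shot trigger box that fires the empty OnTriggered event based on which in-game players' RobotHeroCharacter pawns stand inside it.
; On each begin overlap, IsTriggered checks the overlapping characters against the ICTPGameGameMode player list, requiring someone to be playing.
; MustContainAllPlayers requires every joined player inside; without it the check passes even if none are found, as the loop falls through to true.
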(event `self.ReceiveBeginPlay`)

(event `self.Box.OnComponentBeginOverlap`
  (params (OtherActor :type "Actor Object Reference") (OtherComp :type "PrimitiveComponent Object Reference") (OtherBodyIndex :type Integer) (bFromSweep :type Boolean) (SweepResult :type "HitResult Structure (by ref)"))
  (if (not (`self.HasTriggered`))
    (bind _istriggered (`self.IsTriggered` (`PrimitiveComponent.GetOverlappingActors` (`self.Box`) "/Script/ICTPGame.RobotHeroCharacter")))
    (if _istriggered
      (set `self.HasTriggered` true)
      (`self.OnTriggered`))))

(event `OnTriggered`)

(fn `IsTriggered`
  (params (OverlappingActors :type "Array of Actor Object Reference"))
  (returns (IsTriggered :type Boolean))
  (bind _asictpgame_game_mode (cast `ICTPGameGameMode` (`GameplayStatics.GetGameMode`))
    (:`then`
      (if (`ICTPGameGameMode.IsAnyonePlaying` _asictpgame_game_mode)
        (for _array_element (`ICTPGameGameMode.Players` _asictpgame_game_mode)
          ;[1 1 1] Does the array contain this player?
          (if (`KismetArrayLibrary.Array_Contains` OverlappingActors (`Controller.K2_GetPawn` _array_element))
            ;[1 1 1] We found one player
            (if (`RobotPlayerController.GetIsIn` _array_element)
              (if (not (`self.MustContainAllPlayers`))
                (return true)))
            (else
              ;[1 1 1] Return false if player is in and we have to contain them all
              (if (`RobotPlayerController.GetIsIn` _array_element)
                (if (`self.MustContainAllPlayers`)
                  (return false))))))
        (return true)
        (else
          _)))
    (:`CastFailed`
      _))
  (return false))

(fn `UserConstructionScript`)