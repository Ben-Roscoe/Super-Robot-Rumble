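; AI controller for the Tracker enemy that makes it chase robot hero characters within its sight sphere.
; On possess it caches the pawn, and a looping two-second timer started at BeginPlay runs CheckNewTarget.
; That function picks the overlapping hero closest to the controller's location and stores it as the pawn's FollowedActor.
; It then moves straight toward that actor without pathfinding, using half the melee sphere radius as acceptance radius.
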(event `self.ReceiveBeginPlay`
  (`KismetSystemLibrary.K2_SetTimerDelegate` (delegate `CallCheckNewTarget`) 2.0 true))

(event `CallCheckNewTarget`
  (`self.CheckNewTarget`))

(event `self.OnPossess`
  (params (PossessedPawn :type "Pawn Object Reference"))
  (bind _astracker_enemy_bp (cast `/Game/Blueprints/Enemies/Tracker/TrackerEnemy_BP` PossessedPawn)
    (:`then`
      _)
    (:`CastFailed`
      _))
  (set `self.TrackerPawn` _astracker_enemy_bp))

(fn `CheckNewTarget`
  (bind _trackerpawn (`self.TrackerPawn`))
  (bind _overlappingactors (`PrimitiveComponent.GetOverlappingActors` (`/Game/Blueprints/Enemies/Tracker/TrackerEnemy_BP.SightSphere` _trackerpawn) "/Script/ICTPGame.RobotHeroCharacter"))
  (`/Engine/EditorBlueprintResources/StandardMacros.IsValid` _trackerpawn
    (:`Is Valid`
      (if (> (`KismetArrayLibrary.Array_Length` _overlappingactors) 0)
        (bind _outactor (`/Game/Blueprints/Libraries/Utilities.GetClosestActor` _overlappingactors (`self.K2_GetActorLocation`)))
        (bind _output_get (set `/Game/Blueprints/Enemies/Tracker/TrackerEnemy_BP.FollowedActor` _outactor _trackerpawn))
        (`self.MoveToActor` _output_get (/ (`SphereComponent.SphereRadius` (`/Game/Blueprints/Enemies/Tracker/TrackerEnemy_BP.MeleeSphere` (`self.TrackerPawn`))) 2.0) true false)))))

(fn `UserConstructionScript`)