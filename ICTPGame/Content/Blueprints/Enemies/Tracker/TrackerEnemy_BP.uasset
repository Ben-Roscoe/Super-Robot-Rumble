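; Tracker enemy that zaps its followed actor at melee range and explodes with sound and particles on death.
; The Weapon trigger is pressed at BeginPlay, and each OnFire checks whether FollowedActor overlaps MeleeSphere before applying damage through the game mode.
; A Lightning effect retargets to the victim and shows briefly per hit.
; Construction hides the lightning and registers a dynamic mesh material for damage flashing.
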(event `self.ReceiveBeginPlay`
  (bind _ashealth_bar_ui (cast `/Game/UI/HealthBarUI` (`WidgetComponent.GetUserWidgetObject` (`self.HealthBar`)))
    (:`then`
      (set `/Game/UI/HealthBarUI.OwnerActor` self _ashealth_bar_ui))
    (:`CastFailed`
      _))
  (`WeaponComponent.PressTrigger` (`self.Weapon`))
  (bind _returnvalue (`GameplayStatics.SpawnEmitterAttached` "/Game/Particles/P_PickUp.P_PickUp" (`self.CapsuleComponent`)))
  (`SceneComponent.K2_SetWorldLocation` _returnvalue (`SceneComponent.K2_GetComponentLocation` (`self.CapsuleComponent`)) false false))

(event `self.Health.OnDeath`
  (params (DamageAmount :type "Float (single-precision)") (Instigator :type "Controller Object Reference") (DamageCauser :type "Actor Object Reference"))
  (bind _returnvalue (`GameplayStatics.SpawnEmitterAtLocation` "/Game/Particles/P_Explosion_Blue.P_Explosion_Blue" (`SceneComponent.K2_GetComponentLocation` (`self.Explosion`))))
  (`SceneComponent.SetRelativeScale3D` _returnvalue (* (`SceneComponent.K2_GetComponentScale` (`self.Mesh`)) 0.5))
  (`GameplayStatics.PlaySoundAtLocation` "/Game/Audio/Sounds/Enemy/Enemy_Die_Explode.Enemy_Die_Explode" (`self.K2_GetActorLocation`))
  (`self.K2_DestroyActor`))

(event `self.ReceiveTick`
  (params (DeltaSeconds :type "Float (single-precision)")))

(event `self.Weapon.OnFire`
  (bind _followedactor (`self.FollowedActor`))
  ;[1 1 1] Attacking
  (`/Engine/EditorBlueprintResources/StandardMacros.IsValid` _followedactor
    (:`Is Valid`
      (if (`KismetArrayLibrary.Array_Contains` (`PrimitiveComponent.GetOverlappingActors` (`self.MeleeSphere`) null) _followedactor)
        (bind _asictpgame_game_mode (cast `ICTPGameGameMode` (`GameplayStatics.GetGameMode`)))
        (`ICTPGameGameMode.TryDamage` _asictpgame_game_mode self (`self.FollowedActor`) (`self.ZapDamage`) null)
        (`self.ShootLightning`)
        (`KismetSystemLibrary.Delay` (`self.ZapVisiTime`))
        (`SceneComponent.SetVisibility` (`self.Lightning`) false true)))))

(fn `ShootLightning`
  (bind _lightning (`self.Lightning`))
  (bind _followedactor (`self.FollowedActor`))
  (`/Engine/EditorBlueprintResources/StandardMacros.IsValid` _lightning
    (:`Is Valid`
      (`/Engine/EditorBlueprintResources/StandardMacros.IsValid` _followedactor
        (:`Is Valid`
          (`ParticleSystemComponent.SetActorParameter` _lightning "TargetActor" _followedactor)
          (`SceneComponent.SetVisibility` (`self.Lightning`) true true))))))

(fn `UserConstructionScript`
  (`ParticleSystemComponent.SetActorParameter` (`self.Lightning`) "SourceActor" self)
  (`ParticleSystemComponent.SetActorParameter` (`self.Lightning`) "TargetActor" self)
  (`SceneComponent.SetVisibility` (`self.Lightning`) false false)
  (bind _returnvalue (`PrimitiveComponent.CreateDynamicMaterialInstance` (`self.Mesh`) 0 null))
  (`KismetArrayLibrary.Array_Add` (`/Game/Blueprints/Components/FlashOnDamageComponent_BP.FlashMaterials` (`self.FlashOnDamageComponent_BP`)) _returnvalue))