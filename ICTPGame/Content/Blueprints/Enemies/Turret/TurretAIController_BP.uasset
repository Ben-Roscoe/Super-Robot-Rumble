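; AI controller for the turret enemy that activates it when a robot hero character enters its vision radius and deactivates it when none remain.
; A looping one-second timer checks the overlapping heroes and uses a detection flag so activate and deactivate events fire only on state changes.
; Each tick, it turns the turret toward the closest overlapping hero, flattening Z so the rotation is yaw-only.
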(event `self.ReceiveBeginPlay`
  (`KismetSystemLibrary.K2_SetTimerDelegate` (delegate `CallCheckForActivation`) 1.0 true))

(event `CallCheckForActivation`
  (`self.CheckForActivation`))

(event `self.ReceiveTick`
  (params (DeltaSeconds :type "Float (single-precision)"))
  ;[1 1 1] Face closest player
  (bind _asturret_bp (cast `/Game/Blueprints/Enemies/Turret/Turret_BP` (`self.K2_GetPawn`)))
  (bind _returnvalue (`self.K2_GetActorLocation` _asturret_bp))
  (bind _outactor (`/Game/Blueprints/Libraries/Utilities.GetClosestActor` (`PrimitiveComponent.GetOverlappingActors` (`/Game/Blueprints/Enemies/Turret/Turret_BP.TurretVisionRadius` _asturret_bp) "/Script/ICTPGame.RobotHeroCharacter") _returnvalue))
  (`/Engine/EditorBlueprintResources/StandardMacros.IsValid` _outactor
    (:`Is Valid`
      (bind (_returnvalue_x _returnvalue_y) (`KismetMathLibrary.BreakVector` (`self.K2_GetActorLocation` _outactor)))
      (`/Game/Blueprints/Enemies/Turret/Turret_BP.LookAt` _asturret_bp (`KismetMathLibrary.FindLookAtRotation` (`KismetMathLibrary.MakeVector` (.x _returnvalue) (.y _returnvalue)) (`KismetMathLibrary.MakeVector` _returnvalue_x _returnvalue_y))))))

(fn `CheckForActivation`
  (bind _asturret_bp (cast `/Game/Blueprints/Enemies/Turret/Turret_BP` (`self.K2_GetPawn`)))
  (if (> (`KismetArrayLibrary.Array_Length` (`PrimitiveComponent.GetOverlappingActors` (`/Game/Blueprints/Enemies/Turret/Turret_BP.TurretVisionRadius` _asturret_bp) "/Script/ICTPGame.RobotHeroCharacter")) 0)
    (if (not (`self.IsPlayerDetected`))
      (`/Game/Blueprints/Enemies/Turret/Turret_BP.Event Activate` _asturret_bp)
      (set `self.IsPlayerDetected` true))
    (elif (`self.IsPlayerDetected`)
      (`/Game/Blueprints/Enemies/Turret/Turret_BP.Event Deactivate` _asturret_bp)
      (set `self.IsPlayerDetected` false))))

(fn `UserConstructionScript`)