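; Enemy turret that rises when activated, fires bullets from four barrels and explodes on death.
; A wake timeline raises the capsule and primes the barrels, then presses the Weapon trigger; Deactivate reverses it and releases the trigger.
; Weapon fire events alternate barrel pairs, sharing one recoil timeline scaled to burst interval.
; Tick eases rotation toward the LookAt target, and construction registers dynamic materials for damage flashing.
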(event `LookAt`
  (params (NewDestinationRotation :type "Rotator Structure"))
  (set `self.DestinationRotation` NewDestinationRotation))

(event `self.ReceiveTick`
  (params (DeltaSeconds :type "Float (single-precision)"))
  (`self.SetActorRotation` (`KismetMathLibrary.RInterpTo` (`self.K2_GetActorRotation`) (`self.DestinationRotation`) DeltaSeconds (`self.RotationSpeed`))))

(event `Event Activate`
  ;[1 1 1] Raise Turret
  (bind (_direction _raiseframe _primeturretbarrel1 _primeturretbarrel2 _primeturretbarrel3 _primeturretbarrel4) (`Timeline|TurretWake_Timeline` :`NewTime` 0.0 :!label _label)
    (:`Update`
      (`SceneComponent.K2_SetRelativeLocation` (`self.Capsule`) (`KismetMathLibrary.VLerp` (0.0 0.0 0.0) (0.0 0.0 175.0) _raiseframe) false false)
      (`SceneComponent.K2_SetRelativeLocation` (`self.TurretBarrel4`) (`KismetMathLibrary.VLerp` (0.0 0.0 -120.0) (0.0 40.0 -120.0) _primeturretbarrel1) false false)
      (`SceneComponent.K2_SetRelativeLocation` (`self.TurretBarrel3`) (`KismetMathLibrary.VLerp` (0.0 0.0 -80.0) (0.0 40.0 -80.0) _primeturretbarrel2) false false)
      (`SceneComponent.K2_SetRelativeLocation` (`self.TurretBarrel2`) (`KismetMathLibrary.VLerp` (0.0 0.0 -40.0) (0.0 40.0 -40.0) _primeturretbarrel3) false false)
      (`SceneComponent.K2_SetRelativeLocation` (`self.TurretBarrel1`) (`KismetMathLibrary.VLerp` (0.0 0.0 0.0) (0.0 40.0 0.0) _primeturretbarrel4) false false))
    (:`Finished`
      ;[1 1 1] Fire when setup animation complete
      (if (`|EnumEquality` _direction "Forward")
        (`KismetSystemLibrary.Delay` 0.0)
        (`WeaponComponent.PressTrigger` (`self.Weapon`))))))

(event `Event Deactivate`
  (`|ExecutionSequence`
    (:`then_0`
      (goto _label :!via `Reverse`))
    (:`then_1`
      ;[1 1 1] Raise Turret
      (`WeaponComponent.ReleaseTrigger` (`self.Weapon`)))))

(event `self.ReceiveBeginPlay`
  (bind _ashealth_bar_ui (cast `/Game/UI/HealthBarUI` (`WidgetComponent.GetUserWidgetObject` (`self.HealthBar`)))
    (:`then`
      ;[1 1 1] Match animation to fire rate
      (set `/Game/UI/HealthBarUI.OwnerActor` self _ashealth_bar_ui))
    (:`CastFailed`
      _))
  (`TimelineComponent.SetPlayRate` (`self.1st_3rd_Barrels`) (/ 1.0 (`WeaponComponent.SecondsBetweenBursts` (`self.Weapon`))))
  (set `self.DestinationRotation` (`self.K2_GetActorRotation`)))

(event `self.Weapon.OnFire`
  ;[1 1 1] Firing Bullets and Animation
  (`GameplayStatics.PlaySoundAtLocation` "/Game/Audio/Sounds/Enemy/Turret_Fire_2.Turret_Fire_2" (`self.K2_GetActorLocation`))
  (if (`self.FireSwitch`)
    (`|SpawnActorFromClass` "/Game/Blueprints/Projectiles/TurretBullet_BP2.TurretBullet_BP2_C" (`SceneComponent.K2_GetComponentToWorld` (`self.FirstArrow`)) "Undefined" "OverrideRootScale" null (`self.GetInstigator`))
    (`|SpawnActorFromClass` "/Game/Blueprints/Projectiles/TurretBullet_BP2.TurretBullet_BP2_C" (`SceneComponent.K2_GetComponentToWorld` (`self.ThirdArrow`)) "Undefined" "OverrideRootScale" null (`self.GetInstigator`))
    (bind (_direction _fire) (`Timeline|1st_3rd_Barrels` :!via `PlayFromStart` :!label _label_2)
      (:`Update`
        (if (`self.FireSwitch`)
          (`SceneComponent.K2_SetRelativeLocation` (`self.TurretBarrel1`) (`KismetMathLibrary.VLerp` (0.0 40.0 0.0) (0.0 0.0 0.0) _fire) false false)
          (`SceneComponent.K2_SetRelativeLocation` (`self.TurretBarrel3`) (`KismetMathLibrary.VLerp` (0.0 40.0 -80.0) (0.0 0.0 -80.0) _fire) false false)
          (else
            (`SceneComponent.K2_SetRelativeLocation` (`self.TurretBarrel2`) (`KismetMathLibrary.VLerp` (0.0 40.0 -40.0) (0.0 0.0 -40.0) _fire) false false)
            (`SceneComponent.K2_SetRelativeLocation` (`self.TurretBarrel4`) (`KismetMathLibrary.VLerp` (0.0 40.0 -120.0) (0.0 0.0 -120.0) _fire) false false))))
      (:`Finished`
        (set `self.FireSwitch` (not (`self.FireSwitch`)))))
    (else
      (`|SpawnActorFromClass` "/Game/Blueprints/Projectiles/TurretBullet_BP2.TurretBullet_BP2_C" (`SceneComponent.K2_GetComponentToWorld` (`self.SecondArrow`)) "Undefined" "OverrideRootScale" null (`self.GetInstigator`))
      (`|SpawnActorFromClass` "/Game/Blueprints/Projectiles/TurretBullet_BP2.TurretBullet_BP2_C" (`SceneComponent.K2_GetComponentToWorld` (`self.ForthArrow`)) "Undefined" "OverrideRootScale" null (`self.GetInstigator`))
      (goto _label_2 :!via `PlayFromStart`))))

(event `self.Health.OnDeath`
  (params (DamageAmount :type "Float (single-precision)") (Instigator :type "Controller Object Reference") (DamageCauser :type "Actor Object Reference"))
  (`GameplayStatics.SpawnEmitterAtLocation` "/Game/Particles/P_Explosion_Blue.P_Explosion_Blue" (`SceneComponent.K2_GetComponentLocation` (`self.Capsule`)))
  (`GameplayStatics.PlaySoundAtLocation` "/Game/Audio/Sounds/Enemy/Enemy_Die_Explode.Enemy_Die_Explode" (`self.K2_GetActorLocation`))
  (`self.K2_DestroyActor`))

(fn `UserConstructionScript`
  (for _array_element (`SceneComponent.GetChildrenComponents` (`self.Capsule`) true)
    (bind _asprimitive_component (cast `PrimitiveComponent` _array_element))
    (for _index (range (`PrimitiveComponent.GetNumMaterials` _asprimitive_component))
      (bind _returnvalue (`PrimitiveComponent.CreateDynamicMaterialInstance` _asprimitive_component _index null))
      (`KismetArrayLibrary.Array_Add` (`/Game/Blueprints/Components/FlashOnDamageComponent_BP.FlashMaterials` (`self.FlashOnDamageComponent_BP`)) _returnvalue))))