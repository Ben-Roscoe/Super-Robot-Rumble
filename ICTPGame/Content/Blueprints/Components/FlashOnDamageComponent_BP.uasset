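; Actor component that flashes its owner's materials whenever the owner takes damage.
; It binds to OnTakeAnyDamage at BeginPlay, and each hit restarts a one-shot timer that ends the flash on expiry.
; While flashing, Tick uses the timer's remaining fraction, scaled by a maximum multiplier, to fade a scalar parameter across the FlashMaterials array.
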(event `self.ReceiveBeginPlay`
  (bind _returnvalue (`self.GetOwner`))
  ;[1 1 1] Bind event to owner damage delegate
  (`/Engine/EditorBlueprintResources/StandardMacros.IsValid` _returnvalue
    (:`Is Valid`
      (add `Actor.OnTakeAnyDamage` _returnvalue (delegate `OnOwnerTakeDamage`)))))

(event `OnOwnerTakeDamage`
  (params (Damage :type "Float (double-precision)") (DamageType :type "DamageType Object Reference") (InstigatedBy :type "Controller Object Reference") (DamageCauser :type "Actor Object Reference"))
  (`KismetSystemLibrary.K2_ClearTimerHandle` (`self.FlashTimerHandle`))
  (`self.StartFlash`)
  (bind _returnvalue (`KismetSystemLibrary.K2_SetTimerDelegate` (delegate `OnFlashIntervalEnd`) (`self.FlashInterval`)))
  (set `self.FlashTimerHandle` _returnvalue))

(event `OnFlashIntervalEnd`
  (`self.EndFlash`))

(event `self.ReceiveTick`
  (params (DeltaSeconds :type "Float (single-precision)"))
  (if (`self.IsFlashing`)
    (`self.UpdateFlash`)))

(fn `EndFlash`
  (`self.SetFlashMultipliers` 0.0)
  (set `self.IsFlashing` false))

(fn `SetFlashMultipliers`
  (params (Multiplier :type "Float (double-precision)"))
  (for _array_element (`self.FlashMaterials`)
    (`MaterialInstanceDynamic.SetScalarParameterValue` _array_element (`self.FlashMultiplierParamName`) Multiplier)))

(fn `StartFlash`
  (`self.SetFlashMultipliers` 1.0)
  (set `self.IsFlashing` true))

(fn `UpdateFlash`
  (`self.SetFlashMultipliers` (* (/ (`KismetSystemLibrary.K2_GetTimerRemainingTimeHandle` (`self.FlashTimerHandle`)) (`self.FlashInterval`)) (`self.MaxFlashMultiplier`))))