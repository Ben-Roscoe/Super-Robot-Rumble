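; Door is a double-door Blueprint that opens when a RobotHeroCharacter is inside its sphere trigger while unlocked.
; One timeline swings both panels and slides the base piece on separate tracks, reversing to close.
; It closes when no Characters remain in the sphere, unless forced open.
; ForceOpen, Lock and Unlock events provide external control, with Unlock rechecking current overlaps.
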(event `self.Sphere.OnComponentBeginOverlap`
  (params (OtherActor :type "Actor Object Reference") (OtherComp :type "PrimitiveComponent Object Reference") (OtherBodyIndex :type Integer) (bFromSweep :type Boolean) (SweepResult :type "HitResult Structure (by ref)"))
  (if (and (`self.IsLocked`) (not (`self.IsForcedOpen`))) :!label _label
    (if (and (<= (`KismetArrayLibrary.Array_Length` (`PrimitiveComponent.GetOverlappingActors` (`self.Sphere`) "/Script/Engine.Character")) 0) (not (`self.IsForcedOpen`))) :!label _label_2
      (bind (_direction _dooropentrack _doorbridgetrack) (`Timeline|DoorTimeline` :!via `Reverse` :!label _label_3)
        (:`Update`
          (`SceneComponent.K2_SetRelativeRotation` (`self.RightDoor`) (`KismetMathLibrary.RLerp` (struct) (struct :`Pitch` -90.0) _dooropentrack) false false)
          (`SceneComponent.K2_SetRelativeRotation` (`self.LeftDoor`) (`KismetMathLibrary.RLerp` (struct) (struct :`Pitch` 90.0) _dooropentrack) false false)
          (`SceneComponent.K2_SetRelativeLocation` (`self.DoorBase`) (`KismetMathLibrary.VLerp` (0.0 65.0 0.0) (0.0 0.0 0.0) _doorbridgetrack) false false))))
    (elif (> (`KismetArrayLibrary.Array_Length` (`PrimitiveComponent.GetOverlappingActors` (`self.Sphere`) "/Script/ICTPGame.RobotHeroCharacter")) 0)
      (goto _label_3))))

(event `self.Sphere.OnComponentEndOverlap`
  (params (OtherActor :type "Actor Object Reference") (OtherComp :type "PrimitiveComponent Object Reference") (OtherBodyIndex :type Integer))
  (goto _label_2))

(event `ForceOpen`
  (set `self.IsForcedOpen` true)
  (goto _label_3))

(event `Lock`
  (set `self.IsLocked` true)
  (goto _label_3 :!via `Reverse`))

(event `Unlock`
  (set `self.IsLocked` false)
  (goto _label))

(fn `UserConstructionScript`)